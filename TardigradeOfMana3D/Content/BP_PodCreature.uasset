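; BP_PodCreature is an enemy creature that deals melee-style impact damage to the player.
; AttackCollider's begin overlap caches the player and flags it as in the impact area, while the actor-wide end overlap clears that flag.
; ImpactPlayer, which has no caller in this Blueprint, applies fixed damage to the cached player if the flag is set.
; Debug strings print on overlaps, hits and misses.
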(event OnComponentBeginOverlap(AttackCollider)
  (params (OverlappedComponent :type Primitive%20Component%20Object%20Reference) (OtherActor :type Actor%20Object%20Reference) (OtherComp :type Primitive%20Component%20Object%20Reference) (OtherBodyIndex :type Integer) (bFromSweep :type Boolean) (SweepResult :type Hit%20Result%20Structure%20%28by%20ref%29))
  (bind _asmy_player_character (Utilities|Casting|CastToMyPlayerCharacter OtherActor)
    (:then
      (Variables|Default|SetHitPlayer _asmy_player_character)
      (Development|PrintString "overlap player")
      (Variables|Default|SetInImpactArea true))
    (:CastFailed
      (Development|PrintString "overlap something"))))

(event EventBeginPlay)

(event EventTick
  (params (DeltaSeconds :type Float%20%28single-precision%29)))

(event Collision|EventActorEndOverlap
  (params (OtherActor :type Actor%20Object%20Reference))
  (Utilities|Casting|CastToMyPlayerCharacter OtherActor
    (:then
      (Development|PrintString "end overlap player")
      (Variables|Default|SetInImpactArea false))
    (:CastFailed
      (Development|PrintString "overlap something"))))

(fn ConstructionScript)

(fn ImpactPlayer
  (bind _self self)
  (if (Variables|Default|GetInImpactArea)
    (Development|PrintString "hit player")
    (Variables|Default|SetDamageDealt (Class|MyPlayerCharacter|TakeDamage (Variables|Default|GetHitPlayer) 1e+01 (Utilities|Struct|MakeDamageEvent) (Pawn|GetController _self) _self))
    (else
      (Development|PrintString "missed player"))))